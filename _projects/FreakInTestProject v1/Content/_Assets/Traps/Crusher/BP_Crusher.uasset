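; Crusher trap that looping-animates while on and kills any player overlapping its trigger.
; Activate/deactivate events move the trigger, with timelines driving the animation's play rate for spin-up and spin-down.
; An overlap while on ragdolls the player, starts blood and sound, then reports the death to the game mode after a delay.
; Tick continuously pulls the last victim's pelvis toward the trigger with impulses.
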(event OnComponentBeginOverlap(Trigg)
  (params (OverlappedComponent :type Primitive%20Component%20Object%20Reference) (OtherActor :type Actor%20Object%20Reference) (OtherComp :type Primitive%20Component%20Object%20Reference) (OtherBodyIndex :type Integer) (bFromSweep :type Boolean) (SweepResult :type Hit%20Result%20Structure%20%28by%20ref%29))
  ;[0 0 0] Envia qual player morre
  (bind _asbp_player (Utilities|Casting|CastToBP_Player OtherActor))
  (if (Variables|/Game/_Assets/Traps/Blueprints/BP_GenericTrap.BP_GenericTrap_C|GetOnOff (Variables|Default|GetBP_GenericTrap))
    (if (not (Variables|/Game/Blueprints/BP_Player.BP_Player_C|GetCompletelyDead _asbp_player))
      (Variables|/Game/Blueprints/BP_Player.BP_Player_C|SetCompletelyDead _asbp_player true)
      (Default|ActiveRagdoll _asbp_player)
      (CallFunction|SpawnBlood _asbp_player)
      (Audio|PlaySoundatLocation "/Game/Sounds/Crusher_Bood_SFXCue.Crusher_Bood_SFXCue" "0,0.000000, 0" "0, 0, 0" 1.0 1.0 0.0 0 0 0)
      (Variables|Default|SetPlayer _asbp_player)
      (CallFunction|KillPlayerEvent _asbp_player))))

(event Custom|TurnOff
  ;[0 0 0] TrapAnimation
  (Transformation|SetRelativeLocationAndRotation (Variables|Default|GetTrigg) "0, 0,-80.000000" "0, 0, 0" false false)
  (bind _rollingplayrate (Timeline|CrusherOff PlayFromStart)
    (:Update
      (Components|Timeline|SetPlayRate (Variables|SkeletalMeshActor|GetSkeletalMeshComponent) _rollingplayrate))))

(event Custom|TurnOn
  (bind _skeletalmeshcomponent (Variables|SkeletalMeshActor|GetSkeletalMeshComponent))
  ;[0 0 0] TrapAnimation
  (Transformation|SetRelativeLocationAndRotation (Variables|Default|GetTrigg) "0, 0, 0" "0, 0, 0" false false)
  (Components|Animation|PlayAnimation _skeletalmeshcomponent "/Game/_Assets/Traps/Crusher/Animation/trap_crusher_Anim.trap_crusher_Anim" true)
  (bind _rollingplayrate (Timeline|CrusherOn PlayFromStart)
    (:Update
      (Components|Timeline|SetPlayRate _skeletalmeshcomponent _rollingplayrate))))

(event Custom|KillPlayer_Event
  (params (Player :type BP%20Player%20Object%20Reference))
  ;[1 1 1] Kill Player by time
  (Utilities|FlowControl|Delay (Variables|/Game/Blueprints/BP_Player.BP_Player_C|GetBloodSpawnDuration Player))
  (CallFunction|KillPlayer Player))

(event EventTick
  (params (DeltaSeconds :type Float%20%28single-precision%29))
  (bind _player (Variables|Default|GetPlayer))
  (bind _trigg (Variables|Default|GetTrigg))
  (bind _returnvalue (Transformation|GetWorldLocation _trigg))
  (bind _mesh (Variables|/Script/Engine.Character|GetMesh _player))
  ;[1 1 1] Add Impulse
  (Utilities|IsValid _player
    (:Is%20Valid
      (Physics|AddImpulseatLocation _mesh (* (- (Transformation|GetWorldLocation _mesh) _returnvalue) -1e+02) _returnvalue "Pelvis"))))

(event EventBeginPlay
  ;[1 0.4233 0.9647] Begin Play
  (if (Variables|/Game/_Assets/Traps/Blueprints/BP_GenericTrap.BP_GenericTrap_C|GetOnOff (Variables|Default|GetBP_GenericTrap))
    (CallFunction|Turnon)))

(event EventActivateTrap
  ;[1 0 0] Active/Desactive Trap
  (CallFunction|Turnon))

(event EventDesactivateTrap
  ;[1 0 0] Active/Desactive Trap
  (CallFunction|TurnOff))

(fn ConstructionScript)

(fn SpawnBlood
  (params (self2 :type BP%20Player%20Object%20Reference))
  (if (not (Variables|/Game/Blueprints/BP_Player.BP_Player_C|GetSpawnBloodDecal self2))
    (Variables|/Game/Blueprints/BP_Player.BP_Player_C|SetCanSpawnCrusherParticle? self2 true)
    (Default|SpawnBloodCrusher self2)))

(fn KillPlayer
  (params (Player :type BP%20Player%20Object%20Reference))
  (Class|PlayerState|Died(Message) (Game|GetGameMode) Player))

(fn StopSpawnBlood
  (params (Player :type BP%20Player%20Object%20Reference))
  (if (Variables|/Game/Blueprints/BP_Player.BP_Player_C|GetSpawnBloodDecal Player)
    (Variables|/Game/Blueprints/BP_Player.BP_Player_C|SetCanSpawnCrusherParticle? Player false)
    (Default|SpawnBloodCrusher Player)))