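; Animated saw trap that kills the player on contact, switched through activate/deactivate events and the BPGenericTrap OnOff flag.
; Logic is inverted: activating stops the looping animation, deactivating plays it, and BeginPlay stops it if OnOff is set.
; Tick re-attaches the hit box to the mesh's joint1 socket every frame.
; While OnOff is false, overlap ragdolls and kills the player, spawning a decal and randomized saw sound.
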(event OnComponentBeginOverlap(Box)
  (params (OverlappedComponent :type Primitive%20Component%20Object%20Reference) (OtherActor :type Actor%20Object%20Reference) (OtherComp :type Primitive%20Component%20Object%20Reference) (OtherBodyIndex :type Integer) (bFromSweep :type Boolean) (SweepResult :type Hit%20Result%20Structure%20%28by%20ref%29))
  (bind _asbp_player (Utilities|Casting|CastToBP_Player OtherActor))
  (if (not (Variables|/Game/_Assets/Traps/Blueprints/BP_GenericTrap.BP_GenericTrap_C|GetOnOff (Variables|Default|GetBP_GenericTrap)))
    (Default|SpawnFalledDecal _asbp_player)
    (Default|ActiveRagdoll _asbp_player)
    (Default|DiedEvent _asbp_player)
    (Variables|/Game/Blueprints/BP_Player.BP_Player_C|SetCompletelyDead _asbp_player true)
    (Audio|PlaySoundatLocation "/Game/Sounds/Saw_SFX_Cue.Saw_SFX_Cue" "0, 0, 0" "0, 0, 0" (Math|Random|RandomFloatinRange 0.7 1.3) (Math|Random|RandomFloatinRange 0.7 1.5) 0.0 0 0 0)))

(event Custom|TurnOff
  ;[0 0 0] Trap Animation
  (Audio|Components|Audio|Play (Variables|Default|Getserra_animadaloop) true))

(event Custom|TurnOn
  ;[0 0 0] Trap Animation
  (Audio|Components|Audio|Stop (Variables|Default|Getserra_animadaloop)))

(event EventBeginPlay
  ;[1 0.4233 0.9647] Begin Play
  (if (Variables|/Game/_Assets/Traps/Blueprints/BP_GenericTrap.BP_GenericTrap_C|GetOnOff (Variables|Default|GetBP_GenericTrap))
    (CallFunction|Turnon)))

(event EventTick
  (params (DeltaSeconds :type Float%20%28single-precision%29))
  (Transformation|AttachComponentToComponent (Variables|Default|GetBox) (Variables|Default|Getserra_animadaloop) "joint1" "KeepRelative" "KeepRelative" "KeepRelative" true))

(event EventActivateTrap
  ;[1 0 0] Active/Desactive Trap
  (CallFunction|Turnon))

(event EventDesactivateTrap
  ;[1 0 0] Active/Desactive Trap
  (CallFunction|TurnOff))

(fn ConstructionScript)