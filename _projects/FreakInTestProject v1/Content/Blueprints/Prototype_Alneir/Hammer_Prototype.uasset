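; Prototype hammer pickup that arms BP_Player with a hammer when the player overlaps CanTake while TryGetObject is set.
; While a player is inside InRange, Tick turns Looker toward them and compares yaws against DegreesForGet to judge facing.
; It sends that result and Looker's location to the player, clearing both on exit.
; The tracked player is found by indexing all BP_Player actors with the controller ID.
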(event OnComponentBeginOverlap(InRange)
  (params (OverlappedComponent :type Primitive%20Component%20Object%20Reference) (OtherActor :type Actor%20Object%20Reference) (OtherComp :type Primitive%20Component%20Object%20Reference) (OtherBodyIndex :type Integer) (bFromSweep :type Boolean) (SweepResult :type Hit%20Result%20Structure%20%28by%20ref%29))
  ;[1 1 1] Inside and OutSide of the trigger
  (bind _asbp_player (Utilities|Casting|CastToBP_Player OtherActor))
  (Variables|Default|SetInTrigger? true)
  (bind _asplayer_controller (Utilities|Casting|CastToPlayerController (Pawn|GetController _asbp_player))))

(event OnComponentBeginOverlap(CanTake?)
  (params (OverlappedComponent :type Primitive%20Component%20Object%20Reference) (OtherActor :type Actor%20Object%20Reference) (OtherComp :type Primitive%20Component%20Object%20Reference) (OtherBodyIndex :type Integer) (bFromSweep :type Boolean) (SweepResult :type Hit%20Result%20Structure%20%28by%20ref%29))
  ;[1 1 1] TakeWeapon
  (bind _asbp_player (Utilities|Casting|CastToBP_Player OtherActor))
  (if (Variables|/Game/Blueprints/BP_Player.BP_Player_C|GetTryGetObject _asbp_player)
    (Default|WithNoWeapon _asbp_player)
    (Variables|/Game/Blueprints/BP_Player.BP_Player_C|SetHaveWeapon? _asbp_player true)
    (Variables|/Game/Blueprints/BP_Player.BP_Player_C|SetArmedWithHammer? _asbp_player true)
    (Default|HaveWeaponEvent? _asbp_player)))

(event OnComponentEndOverlap(InRange)
  (params (OverlappedComponent :type Primitive%20Component%20Object%20Reference) (OtherActor :type Actor%20Object%20Reference) (OtherComp :type Primitive%20Component%20Object%20Reference) (OtherBodyIndex :type Integer))
  ;[1 1 1] Inside and OutSide of the trigger
  (bind _asbp_player (Utilities|Casting|CastToBP_Player OtherActor))
  (Variables|Default|SetInTrigger? false)
  (Class|SendWeaponLocation|SendObjectLocation(Message) _asbp_player false "0, 0, 0"))

(event EventTick
  (params (DeltaSeconds :type Float%20%28single-precision%29))
  (bind _looker (Variables|Default|GetLooker))
  ;[1 1 1] Make the actor look for the player
  (if (Variables|Default|GetInTrigger?)
    (Utilities|FlowControl|Sequence
      (:then_0
        (bind _outactors (Actor|GetAllActorsOfClass "/Game/Blueprints/BP_Player.BP_Player_C"))
        (Transformation|SetWorldRotation _looker (Math|Rotator|FindLookatRotation (Transformation|GetWorldLocation _looker) (Transformation|GetWorldLocation (Variables|/Script/Engine.Character|GetMesh (Utilities|Array|Get(acopy) _outactors (Class|GameplayStatics|GetPlayerControllerID (stale OnComponentBeginOverlap(InRange) _asplayer_controller)))))) false false))
      (:then_1
        ;[1 1 1] Get/Set the degree(only Z exes) distance of actors
        (bind _output_get (Variables|Default|SetTryingGet? (>= (Math|Float|Absolute(Float) (- (.Yaw (Math|Rotator|BreakRotator (Transformation|GetActorRotation (Utilities|Array|Get(acopy) _outactors (Class|GameplayStatics|GetPlayerControllerID (stale OnComponentBeginOverlap(InRange) _asplayer_controller)))))) (.Yaw (Math|Rotator|BreakRotator (Transformation|GetWorldRotation (Variables|Default|GetLooker)))))) (Variables|Default|GetDegreesForGet))))
        (Class|SendWeaponLocation|SendObjectLocation(Message) (Utilities|Array|Get(acopy) _outactors (Class|GameplayStatics|GetPlayerControllerID (stale OnComponentBeginOverlap(InRange) _asplayer_controller))) _output_get (Transformation|GetWorldLocation (Variables|Default|GetLooker)))))))

(fn ConstructionScript)