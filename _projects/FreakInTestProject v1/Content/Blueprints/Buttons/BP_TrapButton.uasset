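; BP_TrapButton is a floor-style button that activates a trap when the player overlaps its trigger.
; A press lowers the button mesh, calls TurnOnTrap on the linked BPGenericButton and starts a reset timer.
; If the trap is on when the timer fires, it resets the trap, then re-arms and raises the button after a short delay.
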(event OnComponentBeginOverlap(Trigg)
  (params (OverlappedComponent :type Primitive%20Component%20Object%20Reference) (OtherActor :type Actor%20Object%20Reference) (OtherComp :type Primitive%20Component%20Object%20Reference) (OtherBodyIndex :type Integer) (bFromSweep :type Boolean) (SweepResult :type Hit%20Result%20Structure%20%28by%20ref%29))
  ;[0.5207 1 1] ActiveTrap
  (Utilities|Casting|CastToBP_Player OtherActor)
  (if (not (Variables|Default|GetTriggered))
    (Variables|Default|SetTriggered true)
    (Transformation|SetRelativeLocation (Variables|Default|GetButtonmesh) "0, 0,-35.000000" false false)
    (Default|TurnonTrap (Variables|Default|GetBP_GenericButton))
    ;[1 1 0.2807] UpButton/ResetTRap
    (Utilities|Time|SetTimerbyEvent (delegate Custom|ResetButton) (Variables|Default|GetTimeToReset))))

(event Custom|ResetButton
  (bind _bp_genericbutton (Variables|Default|GetBP_GenericButton))
  ;[1 1 0.2807] UpButton/ResetTRap
  (if (Variables|/Game/Blueprints/Buttons/BP_GenericButton.BP_GenericButton_C|GetTrapOn (Variables|Default|GetBP_GenericButton))
    (Default|ResetButton _bp_genericbutton)
    (Variables|/Game/Blueprints/Buttons/BP_GenericButton.BP_GenericButton_C|SetTrapOn _bp_genericbutton false)
    (Utilities|FlowControl|Delay 2.0)
    (Variables|Default|SetTriggered false)
    (Transformation|SetRelativeLocation (Variables|Default|GetButtonmesh) "0, 0,-25.000000" false false)))

(fn ConstructionScript)