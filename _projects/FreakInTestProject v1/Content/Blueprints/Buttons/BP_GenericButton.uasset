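; Generic button Blueprint that toggles the traps linked to it by a shared TrapNum.
; On BeginPlay it caches actors tagged "Trap"; TurnOnTrap flips each match by sending activate or deactivate messages to its BP_GenericTrap component and actor.
; Matching traps marked Persistent are recorded uniquely, and ResetButton toggles from that list, clearing it inside the loop body after the first toggle.
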(event Custom|ResetButton
  ;[0.399 1 0.4167] ResetTrap
  (Utilities|ResetPersistentTraps))

(event Custom|TurnOnTrap
  ;[1 0.3646 0.3646] Activate Trap
  (Variables|Default|SetTrapOn true)
  (for _array_element (Variables|Default|GetTrapsInGame)
    (CallFunction|GetTrapReferences (Actor|GetComponentbyClass _array_element "/Game/_Assets/Traps/Blueprints/BP_GenericTrap.BP_GenericTrap_C") _array_element)))

(event EventBeginPlay
  (bind _outactors (Actor|GetAllActorswithTag "Trap"))
  (Variables|Default|SetTrapsInGame _outactors))

(fn GetTrapReferences
  (params (Ref_GT :type BP%20Generic%20Trap%20Object%20Reference) (Ref_Trap :type Actor%20Object%20Reference%20%28by%20ref%29))
  (if (== (Variables|/Game/_Assets/Traps/Blueprints/BP_GenericTrap.BP_GenericTrap_C|GetTrapNum Ref_GT) (Variables|Default|GetTrapNum))
    (Utilities|TraponOff Ref_GT Ref_Trap)
    (if (Variables|/Game/_Assets/Traps/Blueprints/BP_GenericTrap.BP_GenericTrap_C|GetPersistent? Ref_GT)
      (Utilities|Array|AddUnique (Variables|Default|GetPersistentTrapAmount) Ref_Trap))))