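; BP_Alavanca is a lever that the player can pull while standing in its trigger area.
; Overlap with a BP_Player enables input on the lever, and ending the overlap disables it.
; Pressing Grab/Throw rotates the lever mesh and sets Triggered, which blocks further pulls.
; ResetLever restores the pose and flag, but the timer meant to call it after TimeToReset is disconnected.
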(event OnComponentBeginOverlap(Trigg)
  (params (OverlappedComponent :type Primitive%20Component%20Object%20Reference) (OtherActor :type Actor%20Object%20Reference) (OtherComp :type Primitive%20Component%20Object%20Reference) (OtherBodyIndex :type Integer) (bFromSweep :type Boolean) (SweepResult :type Hit%20Result%20Structure%20%28by%20ref%29))
  (bind _asbp_player (Utilities|Casting|CastToBP_Player OtherActor))
  (bind _asplayer_controller (Utilities|Casting|CastToPlayerController (Pawn|GetController _asbp_player)))
  (Input|EnableInput _asplayer_controller))

(event OnComponentEndOverlap(Trigg)
  (params (OverlappedComponent :type Primitive%20Component%20Object%20Reference) (OtherActor :type Actor%20Object%20Reference) (OtherComp :type Primitive%20Component%20Object%20Reference) (OtherBodyIndex :type Integer))
  (Input|DisableInput (stale OnComponentBeginOverlap(Trigg) _asplayer_controller)))

(event Custom|ResetLever
  (Variables|Default|SetTriggered false)
  (Transformation|SetRelativeRotation (Variables|Default|GetLeverMesh) "-45.000000, 0, 0" false false))

(event Input|ActionEvents|InputActionGrab/Throw
  (params (Key :type Key%20Structure))
  (:Pressed
    (if (not (Variables|Default|GetTriggered))
      (Transformation|SetRelativeRotation (Variables|Default|GetLeverMesh) "-90.000000, 0, 0" false false)
      (Variables|Default|SetTriggered true))))

(fn ConstructionScript)