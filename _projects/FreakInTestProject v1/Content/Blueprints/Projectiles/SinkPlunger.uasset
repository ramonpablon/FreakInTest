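; Plunger projectile fired by BP_Player that sticks to the bone it hits on another player and staggers or knocks them out.
; In FuckMode it is tinted, shows SuperShot and, unless a fast shot, homes each tick on the desired enemy within range, re-aiming at spine_03.
; Hits reduce FaintingState, or zero it for FuckMode, headshot or airborne victims; zero triggers ragdoll with doubled impulse, otherwise stagger.
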(event Custom|MoveToTarget
  ;[0 0 0] FollowEnemy
  (bind _mytarget (CallFunction|FindHoming))
  (Variables|/Script/Engine.ProjectileMovementComponent|SetHomingTargetComponent (Variables|Default|GetProjectileMovement) _mytarget))

(event Collision|EventHit
  (params (MyComp :type Primitive%20Component%20Object%20Reference) (Other :type Actor%20Object%20Reference) (OtherComp :type Primitive%20Component%20Object%20Reference) (bSelfMoved :type Boolean) (HitLocation :type Vector :default "0, 0, 0") (HitNormal :type Vector :default "0, 0, 0") (NormalImpulse :type Vector :default "0, 0, 0") (Hit :type Hit%20Result%20Structure%20%28by%20ref%29))
  (bind (_bblockinghit _binitialoverlap _time _distance _location _impactpoint _normal _impactnormal _physmat _hitactor _hitcomponent _hitbonename) (Collision|BreakHitResult Hit))
  (bind _returnvalue (Transformation|GetVelocity))
  (bind _returnvalue_2 (Transformation|GetActorLocation))
  (bind _impulseonhit (Variables|Default|GetImpulseOnHit))
  (bind _returnvalue_3 (* _returnvalue _impulseonhit))
  ;[0.3125 0.2871 0.167] ImpulseOnBone
  (Variables|Default|SetHit _bblockinghit)
  (bind _asbp_player (Utilities|Casting|CastToBP_Player Other))
  (Transformation|AttachComponentToComponent (Variables|/Script/Engine.Character|GetMesh _asbp_player) _hitbonename "SnapToTarget" "KeepRelative" "KeepWorld" false)
  (Collision|SetCollisionEnabled (Variables|Default|GetSphere) "NoCollision")
  (Utilities|GetFaintingState _hitbonename _impactnormal _asbp_player
    (:Faint
      (Physics|AddImpulseatLocation (Variables|/Script/Engine.Character|GetMesh _asbp_player) (* _returnvalue_3 2) _returnvalue_2 _hitbonename)
      (Effects|SpawnEmitterAttached "/Game/FX/Particles/Impact/StrongColl.StrongColl" (Variables|/Script/Engine.Character|GetMesh _asbp_player) _hitbonename))
    (:Stangger
      (Physics|AddImpulseatLocation (Variables|/Script/Engine.Character|GetMesh _asbp_player) _returnvalue_3 _returnvalue_2 _hitbonename)
      (Effects|SpawnEmitterAttached "/Game/FX/Particles/Burst/ArrowColl.ArrowColl" (Variables|/Script/Engine.Character|GetMesh _asbp_player) _hitbonename)))
  (Development|SetHiddeninGame (Variables|Default|GetSuperShot) true false))

(event EventBeginPlay
  (bind _instigator (Variables|Actor|GetInstigator))
  ;[1 0.4233 0.9647] Event Tick / Begin Play
  (Collision|IgnoreActorwhenMoving (Variables|Default|GetSphere) _instigator true)
  (bind _asbp_player (Utilities|Casting|CastToBP_Player _instigator))
  (Variables|Default|SetIsFuckMode (Variables|/Game/Blueprints/BP_Player.BP_Player_C|GetFuckMode _asbp_player))
  (Variables|Default|SetIsFastShot (Variables|/Game/Blueprints/BP_Player.BP_Player_C|GetFastShot _asbp_player))
  (Variables|Default|SetRef_DesiredEnemy (Variables|/Game/Blueprints/BP_Player.BP_Player_C|GetDesiredEnemy _asbp_player))
  (Actor|SetLifeSpan 1e+01)
  (if (Variables|Default|GetIsFuckMode)
    (Development|SetHiddeninGame (Variables|Default|GetSuperShot) false false)
    (Rendering|Material|SetVectorParameterValueonMaterials (Variables|Default|Getdesentupidor) "Color" "1.000000,0.095307, 0")))

(event EventTick
  (params (DeltaSeconds :type Float%20%28single-precision%29))
  ;[1 0.4233 0.9647] Event Tick / Begin Play
  (if (not (Variables|Default|GetHit))
    (CallFunction|MovetoTarget)))

(fn ConstructionScript)

(fn FindHoming
  (bind _returnvalue (Transformation|GetActorLocation))
  (bind _ref_desiredenemy (Variables|Default|GetRef_DesiredEnemy))
  (if (not (Variables|Default|GetIsFastShot))
    (Utilities|IsValid _ref_desiredenemy
      (:Is%20Valid
        (if (< (Math|Vector|Distance(Vector) _returnvalue (Transformation|GetActorLocation _ref_desiredenemy)) (Variables|Default|GetclosestDistance))
          (if (Variables|Default|GetIsFuckMode)
            (Utilities|FuckModeon _returnvalue _ref_desiredenemy)
            (return (Variables|/Script/Engine.Actor|GetRootComponent _ref_desiredenemy))))))))