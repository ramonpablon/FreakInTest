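; Game mode for a local multiplayer last-player-standing match with weapon pickups, a countdown and a toxic cloud.
; BeginPlay spawns and possesses players at index-tagged PlayerStarts, activates random weapon spawners and adds the timer widget.
; Tick respawns weapons below a visible cap and runs the Delay-based countdown that triggers the cloud.
; Deaths reset camera aim; one survivor stops the cloud, faces the camera to emote and gets the post-game menu.
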(event Custom|TimeToSpawn
  (bind _avliablespawner (Variables|WeaponSpawners|GetAvliableSpawner))
  ;[0.8923 0 1 0.426] Weapon Spawner Behaviour
  ;;[0.2 0.3 1] Weapon Spawner Timer
  (if (Variables|WeaponSpawners|GetCanSpawn)
    (Variables|WeaponSpawners|SetWeaponTimer (+ (Utilities|Time|GetWorldDeltaSeconds) (Variables|WeaponSpawners|GetWeaponTimer)))
    (if (>= (Variables|WeaponSpawners|GetWeaponTimer) (Variables|WeaponSpawners|GetWeaponRespawnTime))
      (Variables|WeaponSpawners|SetWeaponTimer 0.0)
      (Default|Spawn (Utilities|Array|Get(acopy) _avliablespawner (Math|Random|RandomInteger (Utilities|Array|Length _avliablespawner)))))))

(event Custom|ShowSpawner
  (params (Spawner :type Weapon%20Spawner%20Object%20Reference%20%28by%20ref%29))
  ;[0.8923 0 1 0.426] Weapon Spawner Behaviour
  ;;[1 0.6 0.5] Show Hide Spawners In Game
  (Utilities|Array|Add (Variables|WeaponSpawners|GetVisibleSpawner) Spawner)
  (Utilities|Array|RemoveItem (Variables|WeaponSpawners|GetAvliableSpawner) Spawner))

(event Custom|HideSpawner
  (params (Spawner :type Weapon%20Spawner%20Object%20Reference%20%28by%20ref%29))
  ;[0.8923 0 1 0.426] Weapon Spawner Behaviour
  ;;[1 0.6 0.5] Show Hide Spawners In Game
  (Utilities|Array|RemoveItem (Variables|WeaponSpawners|GetVisibleSpawner) Spawner)
  (Utilities|Array|Add (Variables|WeaponSpawners|GetAvliableSpawner) Spawner))

(event Custom|TimerTIck
  ;[0 1 0.2227] Timer
  (if (and (== (Variables|Default|GetTime%20Sec) 0) (== (Variables|Default|GetTime%20min) 0))
    ;[0 1 0.0242] ToxicCloud Start
    (if (not (Variables|Default|GetToxicCloudStarted))
      (bind _outactors (Actor|GetAllActorsOfClass "/Game/FX/ToxicCloud/ToxicCloud_Actor.ToxicCloud_Actor_C"))
      (Class|SendToxicCloud|SendToxicCloud(Message) (Utilities|Array|Get(acopy) _outactors) true)
      (Variables|Default|SetToxicCloudStarted true))
    (else
      (Utilities|FlowControl|Delay 1.0)
      (Variables|Default|SetTime%20Sec (- (Variables|Default|GetTime%20Sec) 1))
      (if (and (<= (- (Variables|Default|GetTime%20Sec) 1) 0) (> (Variables|Default|GetTime%20min) 0))
        (Variables|Default|SetTime%20min (- (Variables|Default|GetTime%20min) 1))
        (Variables|Default|SetTime%20Sec 59)))))

(event Custom|Win%20Window
  (bind _playeringame (Variables|Game|GetPlayerInGame))
  (bind _returnvalue (Utilities|Array|Length _playeringame))
  (bind _returnvalue_2 (- _returnvalue 1))
  (bind _output (Utilities|Array|Get(acopy) _playeringame _returnvalue_2))
  (bind _my_id (Variables|/Game/Blueprints/BP_Player.BP_Player_C|GetMy_ID _output))
  ;[1 1 1] Win Window
  (if (== (Variables|Default|GetPlayerVivos) 1)
    (Variables|Default|SetDraw false)
    (Variables|/Game/Blueprints/BP_Player.BP_Player_C|SetIsEmote? _output true)
    (Default|WithNoWeapon _output)
    (Transformation|SetActorRotation _output (Math|Rotator|MakeRotator 0.0 0.0 (.yaw (Math|Rotator|FindLookatRotation (Transformation|GetActorLocation _output) (Transformation|GetWorldLocation (Variables|/Game/Blueprints/BP_Camera.BP_Camera_C|GetCamera (Variables|Game|GetRef_Camera)))))))
    (Pawn|Components|CharacterMovement|SetMovementMode (Variables|/Script/Engine.Character|GetCharacterMovement _output) "MOVE_None" 0)
    (bind _outactors (Actor|GetAllActorsOfClass "/Game/FX/ToxicCloud/ToxicCloud_Actor.ToxicCloud_Actor_C"))
    (Variables|/Game/FX/ToxicCloud/ToxicCloud_Actor.ToxicCloud_Actor_C|SetToxicCloudStart (Utilities|Array|Get(acopy) _outactors) false)
    (bind _returnvalue_3 (UserInterface|CreateWidget "/Game/Blueprints/GUI/postGameMenu.postGameMenu_C" (Game|GetPlayerController _my_id)))
    (UserInterface|Viewport|AddtoViewport _returnvalue_3 0)
    (Input|SetInputModeUIOnly (Game|GetPlayerController _my_id) (Variables|/Game/Blueprints/GUI/postGameMenu.postGameMenu_C|GetRestart _returnvalue_3) "DoNotLock")
    (if (Variables|Default|GetDraw)
      (Variables|Default|SetPlayerPauseIndex 0)
      (else
        (Variables|Default|SetPlayerPauseIndex _my_id)))))

(event EventBeginPlay
  ;[1 0.4233 0.9647] Begin Play / Tick
  (CallFunction|GetSpawnPlayers)
  (CallFunction|SpawnPlayers)
  (CallFunction|GetAvaliableSpawners)
  ;[0.7885 1 0] UI Timer
  (bind _returnvalue (UserInterface|CreateWidget "/Game/_Assets/UI/Timer.Timer_C"))
  (UserInterface|Viewport|AddtoViewport _returnvalue 0)
  (Development|ExecuteConsoleCommand "stat fps" 0)
  (bind _outactors (Actor|GetAllActorsOfClass "/Game/Blueprints/BP_Camera.BP_Camera_C"))
  (Variables|Game|SetRef_Camera (Utilities|Array|Get(acopy) _outactors)))

(event EventDied
  (params (Player :type BP%20Player%20Object%20Reference))
  ;[0 0 0] Player Die
  (if (Variables|/Game/Blueprints/BP_Player.BP_Player_C|GetCompletelyDead Player)
    (Utilities|DestroyActor Player)
    (bind _outactors (Actor|GetAllActorsOfClass "/Game/Blueprints/BP_Player.BP_Player_C"))
    (bind _output_get (Variables|Game|SetPlayerInGame _outactors))
    (Default|ResetEnemyList _output_get)
    (Utilities|ResetCameraAim)
    (Variables|Game|SetKill%20Z false)
    (CallFunction|WinWindow)))

(event EventTick
  (params (DeltaSeconds :type Float%20%28single-precision%29))
  ;[1 0.4233 0.9647] Begin Play / Tick
  (CallFunction|SpawnifPossible)
  (CallFunction|TimerTIck))

(fn ConstructionScript)

(fn SpawnPlayers
  (for _index (range 0 (- (Variables|SpawnPlayers|GetMaxPlayerCount) 1))
    (Variables|SpawnPlayers|SetIndex _index)
    ;[0 0 0] Para cada for
    (for _array_element (Variables|SpawnPlayers|GetPlayerStartCount)
      (if (Utilities|Name|Equal(Name) (Variables|/Script/Engine.PlayerStart|GetPlayerStartTag _array_element) (Utilities|String|StringToName (Utilities|String|ToString(Integer) (Variables|SpawnPlayers|GetIndex))))
        (Class|GameplayStatics|CreatePlayer (Variables|SpawnPlayers|GetIndex))
        (bind _returnvalue (Game|SpawnActorfromClass "/Game/Blueprints/BP_Player.BP_Player_C" (Transformation|GetActorTransform _array_element) "Undefined" 0 0))
        (Pawn|Possess (Game|GetPlayerController (Variables|SpawnPlayers|GetIndex)) _returnvalue)
        (Utilities|Array|AddUnique (Variables|SpawnPlayers|GetStartPlayers) _returnvalue))))
  (Variables|Game|SetPlayerInGame (Variables|SpawnPlayers|GetStartPlayers)))

(fn GetAvaliableSpawners
  (bind _outactors (Actor|GetAllActorsOfClass "/Game/Blueprints/Weapons/WeaponSpawner.WeaponSpawner_C"))
  (bind _output_get (Variables|Game|SetWeaponSpawners _outactors))
  (for _array_element _output_get
    (Rendering|SetActorHiddenInGame _array_element true)
    (Utilities|Array|Add (Variables|WeaponSpawners|GetAvliableSpawner) _array_element))
  ;[0 0 0] Select Start Spawnrs
  (Utilities|FlowControl|ForLoopwithBreak 0 (Variables|WeaponSpawners|GetMaxSpawnNum)
    (:LoopBody
      (LocalVariables|SetCurrentSpawner (Math|Random|RandomInteger (Utilities|Array|Length (Variables|WeaponSpawners|GetAvliableSpawner))))
      (if (not (Utilities|Array|ContainsItem (LocalVariables|GetStartSpawner) (LocalVariables|GetCurrentSpawner)))
        (Utilities|Array|Add (LocalVariables|GetStartSpawner) (LocalVariables|GetCurrentSpawner))))
    (:Completed
      ;[0 0 0] Spawn Spawners
      (for _array_element_2 (LocalVariables|GetStartSpawner)
        (Utilities|IsValid (Utilities|Array|Get(acopy) (Variables|WeaponSpawners|GetAvliableSpawner) _array_element_2)
          (:Is%20Valid
            (Default|Spawn (Utilities|Array|Get(acopy) (Variables|WeaponSpawners|GetAvliableSpawner) _array_element_2))))))))

(fn GetSpawnPlayers
  ;[0 0 0] Get Player Start Point
  (bind _outactors (Actor|GetAllActorsOfClass "/Script/Engine.PlayerStart"))
  (Variables|SpawnPlayers|SetPlayerStartCount _outactors))

(fn SpawnifPossible
  (Variables|WeaponSpawners|SetCanSpawn (< (Utilities|Array|Length (Variables|WeaponSpawners|GetVisibleSpawner)) (Variables|WeaponSpawners|GetMaxSpawnNum)))
  (CallFunction|TimetoSpawn))