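; Game mode for local multiplayer that creates players, gives each an EmptyPawn and points them at a shared BP_Camera.
; Spawn events switch controllers between Freak, Gost and EmptyPawn, at the current pawn's position or a random PlayerStart, and Freak/Gost spawns update FreaksInGame.
; Random starts come from PSNonAvaliable, which holds free starts despite its name.
; PlayerStart use is tracked in arrays, with a delayed reset pool processed from Tick.
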(event EventTick
  (params (DeltaSeconds :type Float%20%28single-precision%29))
  (CallFunction|Debug)
  ;[1 1 1] respwnar quem tem que reespanar
  (|RespawnPlayerStart))

(event EventBeginPlay
  (GameComponents|GetGameCamera)
  (GameComponents|GetAllPlayerStart)
  (GameComponents|SpawnEmptyPawns)
  (CallFunction|SetFreakControllersinGame))

(fn ConstructionScript)

(fn GetAllPlayerStart
  (bind _outactors (Actor|GetAllActorsOfClass "/Script/Engine.PlayerStart"))
  (bind _output_get (Variables|SpawnPlayers|SetPlayerStartCount _outactors))
  ;[1 1 1] adiciona os PS que spawnaram no "em uso"
  (Variables|RandomPlayerStart|SetPSNonAvaliable _output_get))

(fn SpawnEmptyPawns
  (while (<= (Variables|SpawnPlayers|GetControllersInGame) (Variables|SpawnPlayers|GetMaxPlayerIndex))
    (Class|GameplayStatics|CreatePlayer -1)
    (Variables|SpawnPlayers|SetControllersInGame (+ (Variables|SpawnPlayers|GetControllersInGame) 1)))
  (for _index (range 1 (Variables|SpawnPlayers|GetControllersInGame))
    (bind _returnvalue (Utilities|MyPSIndex))
    (bind _returnvalue_2 (Game|SpawnActorfromClass "/Game/_Blueprints/EmptyPawn.EmptyPawn_C" _returnvalue "AlwaysSpawn" 0 0))
    (Pawn|Possess (Game|GetPlayerController (- _index 1)) _returnvalue_2)
    (Game|Player|SetViewTargetwithBlend (Game|GetPlayerController (- _index 1)) (Variables|GameComponents|GetMainCamera) 0.0 "VTBlend_Linear" 0.0 false)
    (Utilities|AddPSinUse))
  (Development|PrintString (Utilities|String|Append (Utilities|String|ToString(Integer) (Variables|SpawnPlayers|GetControllersInGame)) " freak controllers foram instanciados") true true "(R=1.000000,G=0.384861,B=0.374913,A=1.000000)"))

(fn Debug
  (for _array_element (Variables|RandomPlayerStart|GetPSPoolToReset)
    (Development|PrintString (Utilities|String|Append (Utilities|GetDisplayName _array_element) " in the pool") true true "(R=1.000000,G=0.818872,B=0.000000,A=1.000000)" 0.0)))

(fn GetGameCamera
  (bind _outactors (Actor|GetAllActorsOfClass "/Game/_Blueprints/BP_Camera.BP_Camera_C"))
  (Variables|GameComponents|SetMainCamera (Utilities|Array|Get(acopy) _outactors)))

(fn SetFreakControllersinGame
  (bind _outactors (Actor|GetAllActorsOfClass "/Game/_Blueprints/FreakController.FreakController_C"))
  (Variables|Default|SetFreakControllersInGame _outactors))

(fn FraksinGameSetup
  (params (Freak :type Freak%20Object%20Reference%20%28by%20ref%29) (Add%20/Remove :type Boolean))
  (bind _freaksingame (Variables|Default|GetFreaksInGame))
  (if Add%20/Remove
    (Utilities|Array|AddUnique _freaksingame Freak)
    (else
      (Utilities|Array|RemoveItem _freaksingame Freak))))

(event Custom|SpawnGost
  (params (PlayerController :type Player%20Controller%20Object%20Reference) (In%20Death%20Postion :type Boolean))
  (bind _returnvalue (Pawn|GetControlledPawn PlayerController))
  (Utilities|IsValid _returnvalue
    (:Is%20Valid
      (Utilities|SetFreakSpawnPosition In%20Death%20Postion _returnvalue)
      (bind _returnvalue_2 (Game|SpawnActorfromClass "/Game/_Blueprints/Gost/Gost.Gost_C" (Variables|RandomPlayerStart|GetSpawnPosition) "AlwaysSpawn" 0 0))
      (CallFunction|FraksinGameSetup (.AsFreak (Utilities|Casting|CastToFreak _returnvalue)) false)
      (Pawn|Possess PlayerController _returnvalue_2)
      (Game|Player|SetViewTargetwithBlend PlayerController (Variables|GameComponents|GetMainCamera) 0.0 "VTBlend_Linear" 0.0 false)
      (return))))

(event Custom|SpawnFreak
  (params (PlayerController :type Freak%20Controller%20Object%20Reference) (InDeathPosition? :type Boolean))
  (bind _returnvalue (Pawn|GetControlledPawn PlayerController))
  (Utilities|IsValid _returnvalue
    (:Is%20Valid
      (Utilities|SetFreakSpawnPosition InDeathPosition? _returnvalue)
      (CallFunction|FraksinGameSetup (.AsFreak (Utilities|Casting|CastToFreak _returnvalue)) false)
      (Actor|DestroyActor _returnvalue)
      (bind _returnvalue_2 (Game|SpawnActorfromClass "/Game/_Blueprints/Freak.Freak_C" (Variables|RandomPlayerStart|GetSpawnPosition) "AlwaysSpawn" 0 0))
      (CallFunction|FraksinGameSetup _returnvalue_2 true)
      (Pawn|Possess PlayerController _returnvalue_2)
      (Game|Player|SetViewTargetwithBlend PlayerController (Variables|GameComponents|GetMainCamera) 0.0 "VTBlend_Linear" 0.0 false)
      (return))))

(event Custom|DespawnCharacter
  (params (PlayerController :type Player%20Controller%20Object%20Reference) (InDeathPosition? :type Boolean))
  (bind _returnvalue (Pawn|GetControlledPawn PlayerController))
  (Utilities|IsValid _returnvalue
    (:Is%20Valid
      (Utilities|SetFreakSpawnPosition InDeathPosition? _returnvalue)
      (Actor|DestroyActor _returnvalue)
      (bind _returnvalue_2 (Game|SpawnActorfromClass "/Game/_Blueprints/EmptyPawn.EmptyPawn_C" (Variables|RandomPlayerStart|GetSpawnPosition) "AlwaysSpawn" 0 0))
      (Pawn|Possess PlayerController _returnvalue_2)
      (Game|Player|SetViewTargetwithBlend PlayerController (Variables|GameComponents|GetMainCamera) 0.0 "VTBlend_Linear" 0.0 false)
      (return))))