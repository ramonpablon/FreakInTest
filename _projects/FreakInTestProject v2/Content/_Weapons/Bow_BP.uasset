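; Bow weapon Blueprint that shows particle effects on its Cylinder component as the bow moves through three stages and fires.
; Stage 1 attaches a looping-style water ball tracked as CurrentParticle, and Stage 2 adds a temporary water hit burst.
; Stage 3 swaps the tracked particle for a thunder ball plus a timed hit burst.
; ShotEvent destroys whichever tracked particle is active.
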(event Custom|BowStage3
  ;[1 1 1] Comment
  (Components|DestroyComponent (Variables|Default|GetCurrentParticle))
  (bind _returnvalue (Effects|SpawnEmitterAttached "/Game/FXVarietyPack/Particles/P_ky_thunderBall.P_ky_thunderBall" (Variables|Default|GetCylinder) "None" "0, 0, 0" "0, 0, 0" "1.000000,1.000000,1.000000" "SnapToTarget" true "AutoRelease"))
  (Variables|Default|SetCurrentParticle _returnvalue)
  (bind _returnvalue_2 (Effects|SpawnEmitterAttached "/Game/FXVarietyPack/Particles/P_ky_ThunderBallHit.P_ky_ThunderBallHit" (Variables|Default|GetCylinder) "None" "0, 0, 0" "0, 0, 0" "1.000000,1.000000,1.000000" "SnapToTarget" true "AutoRelease"))
  (Utilities|FlowControl|Delay 2.0)
  (Components|DestroyComponent _returnvalue_2))

(event Custom|BowStage1
  ;[1 1 1] Comment
  (bind _returnvalue (Effects|SpawnEmitterAttached "/Game/FXVarietyPack/Particles/P_ky_waterBall.P_ky_waterBall" (Variables|Default|GetCylinder) "None" "0, 0, 0" "0, 0, 0" "1.000000,1.000000,1.000000" "SnapToTarget" true "AutoRelease"))
  (Variables|Default|SetCurrentParticle _returnvalue))

(event Custom|ShotEvent
  (bind _currentparticle (Variables|Default|GetCurrentParticle))
  (Utilities|IsValid _currentparticle
    (:Is%20Valid
      (Components|DestroyComponent _currentparticle))))

(event Custom|BowStage2
  ;[1 1 1] Comment
  (bind _returnvalue (Effects|SpawnEmitterAttached "/Game/FXVarietyPack/Particles/P_ky_waterBallHit.P_ky_waterBallHit" (Variables|Default|GetCylinder) "None" "0, 0, 0" "0, 0, 0" "1.000000,1.000000,1.000000" "SnapToTarget" true "AutoRelease"))
  (Utilities|FlowControl|Delay 2.0)
  (Components|DestroyComponent _returnvalue))

(fn ConstructionScript)